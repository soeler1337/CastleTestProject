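; BP_Interactable is an outfit pickup that the player can focus on and interact with.
; The construction script applies the Outfit variable to its skeletal mesh.
; Focus shows the widget and uses a short retriggerable delay to hide it once Focus calls stop arriving.
; Interact passes the displayed mesh to player character 0 through SetOutfitMessage, then destroys the actor.
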(event EventFocus
  (Development|SetHiddeninGame (Variables|Default|GetWidget) false false)
  (Utilities|FlowControl|RetriggerableDelay 0.1)
  (Development|SetHiddeninGame (Variables|Default|GetWidget) true false))

(event EventInteract
  (Class|BPIInteraction|SetOutfit(Message) (Game|GetPlayerCharacter 0) (Components|SkeletalMesh|GetSkeletalMeshAsset (Variables|Default|GetSkeletalMesh)))
  (Actor|DestroyActor))

(fn ConstructionScript
  (Components|SkeletalMesh|SetSkeletalMeshAsset (Variables|Default|GetSkeletalMesh) (Variables|Default|Getoutfit)))