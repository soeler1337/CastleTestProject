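; BP_Tor is a metal gate actor that slides vertically open and closed through its Open/Close event.
; A timeline drives a lerp on the gate mesh's relative Z location, raising it from its origin to the open position.
; The Geschlossen flag chooses between playing and reversing the timeline, and updates only when the timeline finishes, based on its direction.
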(event Custom|Open/Close
  (if (Variables|Default|Getgeschlossen?)
    (bind (_direction _time_float) (Timeline|Timeline Play)
      (:Update
        (Transformation|SetRelativeLocation (Variables|Default|GetSM_MetalGate04 self) (Math|Vector|Lerp(Vector) "0.0,0.0,0.0" (Math|Vector|MakeVector 0.0 0.0 3e+02) _time_float) false false))
      (:Finished
        (switch Utilities|FlowControl|Switch|SwitchonETimelineDirection _direction
          (:Forward
            (Variables|Default|Setgeschlossen? false))
          (:Backward
            (Variables|Default|Setgeschlossen? true)))))
    (else
      (Timeline|Timeline Reverse))))

(event EventBeginPlay
  (Components|Timeline|SetPlayRate (Variables|Default|GetTimeline) 1.0))

(fn ConstructionScript)