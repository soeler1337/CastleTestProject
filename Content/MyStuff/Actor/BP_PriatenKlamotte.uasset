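; BP_PriatenKlamotte is an interactable clothing pickup that gives the player an outfit.
; Focus shows its widget and restarts a short retriggerable delay, so the widget hides itself once focus calls stop arriving.
; Interact passes the actor's skeletal mesh asset to the player character through a Set Outfit message, then destroys the actor.
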(event EventInteract
  (params (player :type BP%20Third%20Person%20Character%20Object%20Reference))
  (Class|BPIThirdPerson|SetOutfit(Message) (Game|GetPlayerCharacter 0) (Components|SkeletalMesh|GetSkeletalMeshAsset (Variables|Default|GetSkeletalMesh)))
  (Actor|DestroyActor))

(event EventFocus
  (Development|SetHiddeninGame (Variables|Default|GetWidget) false false)
  (Utilities|FlowControl|RetriggerableDelay 0.1)
  (Development|SetHiddeninGame (Variables|Default|GetWidget) true false))

(fn ConstructionScript)